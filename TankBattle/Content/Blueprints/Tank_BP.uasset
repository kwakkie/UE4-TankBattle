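; Tank pawn Blueprint that sets up the turret and barrel and handles orbit camera aiming.
; On BeginPlay it passes the Turret and Barrel components to their child actor setters.
; The AimAzimuth axis yaws the azimuth gimbal and AimElevation pitches the camera boom, keeping the two rotations on separate components.
; Both rotations are local and scaled by world delta seconds for frame-rate independence.
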(event `self.ReceiveBeginPlay`
  (`self.SetTurretChildActor` (`self.Turret`))
  (`self.SetBarrelChildActor` (`self.Barrel`)))

(event `InputAxis|AimAzimuth`
  (params (AxisValue :type "Float (single-precision)"))
  ;[1 1 1] Camera input binding - AimAzimuth left/right - AimElevation up/down
  (`SceneComponent.K2_AddLocalRotation` (`self.Azimuth GImbal`) (`KismetMathLibrary.MakeRotator` 0.0 0.0 (* AxisValue (`GameplayStatics.GetWorldDeltaSeconds`) 100.0)) false false))

(event `InputAxis|AimElevation`
  (params (AxisValue :type "Float (single-precision)"))
  ;[1 1 1] Camera input binding - AimAzimuth left/right - AimElevation up/down
  (`SceneComponent.K2_AddLocalRotation` (`self.Camera_Boom`) (`KismetMathLibrary.MakeRotator` 0.0 (* AxisValue (`GameplayStatics.GetWorldDeltaSeconds`) 100.0)) false false))

(fn `UserConstructionScript`)